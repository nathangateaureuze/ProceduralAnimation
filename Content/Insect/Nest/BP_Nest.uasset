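; Insect nest that spawns a roaming insect 3 seconds after BeginPlay and sets the same timer again whenever OnInsectDie fires.
; Spawning respects a maximum count and uses random reachable navmesh points within the nest radius, retrying after a short delay on failure.
; Each insect gets a nest reference plus randomly picked body parts and two colors from the nest's arrays.
; The construction script draws the spawn radius as a debug sphere.
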(event `self.ReceiveBeginPlay`
  (`KismetSystemLibrary.FlushPersistentDebugLines`)
  (`KismetSystemLibrary.K2_SetTimerDelegate` (delegate `SpawnInsect`) 3.0))

(event `SpawnInsect`
  (bind (_color1 _color2) (`self.GetRandomColors`))
  (bind (_randomlocation _returnvalue) (`NavigationSystemV1.K2_GetRandomReachablePointInRadius` (`SceneComponent.K2_GetComponentLocation` (`self.NestMesh`)) (`self.SpawnerZoneRadius`) null "/Game/Insect/AI/NQF_Test.NQF_Test_C"))
  (if (< (`self.CurrentNbInsect`) (`self.MaxNbInsect`))
    (if _returnvalue :!label _label
      (`|SpawnActorFromClass` "/Game/Insect/BP_Insect_Roaming.BP_Insect_Roaming_C" (`KismetMathLibrary.MakeTransform` _randomlocation) "Undefined" "MultiplyWithRoot" null self (`self.GetRandomAbdomen`) (`self.GetRandomThorax`) (`self.GetRandomHead`) (`self.GetRandomAntennae`) (`self.GetRandomLeg`) _color1 _color2 null)
      (set `self.CurrentNbInsect` (+ (`self.CurrentNbInsect`) 1))
      (else
        (`KismetSystemLibrary.PrintString` "Unreachable" true true (struct :`R` 1.0 :`A` 1.0))
        (`KismetSystemLibrary.Delay` 0.2)
        (goto _label)))))

(event `OnInsectDie`
  (params (InsectRef :type "/Game/Insect/BP_Insect Object Reference"))
  (set `self.CurrentNbInsect` (- (`self.CurrentNbInsect`) 1))
  (`KismetSystemLibrary.K2_SetTimerDelegate` (delegate `SpawnInsect`) 3.0))

(fn `GetRandomAbdomen`
  (returns (Abdomen :type "/Game/Insect/Members/Abdomen/AbdomenDA Object Reference"))
  (bind _abdomens (`self.Abdomens`))
  (return (`|GetArrayItem` _abdomens (`KismetMathLibrary.RandomInteger` (`KismetArrayLibrary.Array_Length` _abdomens)))))

(fn `GetRandomAntennae`
  (returns (Antennae :type "/Game/Insect/Members/Antennae/AntennaeDA Object Reference"))
  (bind _antennaes (`self.Antennaes`))
  (return (`|GetArrayItem` _antennaes (`KismetMathLibrary.RandomInteger` (`KismetArrayLibrary.Array_Length` _antennaes)))))

(fn `GetRandomColors`
  (returns (Color1 :type "/Game/Insect/Colors/ColorDA Object Reference") (Color2 :type "/Game/Insect/Colors/ColorDA Object Reference"))
  (bind _colors (`self.Colors`))
  (bind _returnvalue (`KismetMathLibrary.RandomInteger` (`KismetArrayLibrary.Array_Length` _colors)))
  (return (`|GetArrayItem` _colors _returnvalue) (`|GetArrayItem` _colors _returnvalue)))

(fn `GetRandomHead`
  (returns (Head :type "/Game/Insect/Members/Head/HeadDA Object Reference"))
  (bind _heads (`self.Heads`))
  (return (`|GetArrayItem` _heads (`KismetMathLibrary.RandomInteger` (`KismetArrayLibrary.Array_Length` _heads)))))

(fn `GetRandomLeg`
  (returns (Leg :type "/Game/Insect/Members/Leg/LegDA Object Reference"))
  (bind _legs (`self.Legs`))
  (return (`|GetArrayItem` _legs (`KismetMathLibrary.RandomInteger` (`KismetArrayLibrary.Array_Length` _legs)))))

(fn `GetRandomThorax`
  (returns (Thorax :type "/Game/Insect/Members/Thorax/ThoraxDA Object Reference"))
  (bind _thoraxes (`self.Thoraxes`))
  (return (`|GetArrayItem` _thoraxes (`KismetMathLibrary.RandomInteger` (`KismetArrayLibrary.Array_Length` _thoraxes)))))

(fn `UserConstructionScript`
  (`KismetSystemLibrary.FlushPersistentDebugLines`)
  (`KismetSystemLibrary.DrawDebugSphere` (`SceneComponent.K2_GetComponentLocation` (`self.NestMesh`)) (`self.SpawnerZoneRadius`) 12 (struct :`R` 1.0 :`B` 1.0 :`A` 1.0) 9999999999999.0 4.0))