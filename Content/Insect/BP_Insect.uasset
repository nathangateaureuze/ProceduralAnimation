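; BP_Insect is a modular insect actor assembled from body-part data: abdomen, thorax, head, antennae and six three-segment legs as static meshes.
; The construction script assigns the meshes; on Control Rig pre-initialize, parts are detached and reset, and their socket transforms feed CR_Insect.
; A few ticks after the first forward solve, each part snaps to its skeleton socket, with left-side parts mirrored by negative scale and flipped rotations.
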(event `self.ReceiveBeginPlay`)

(event `self.ControlRig.OnPreInitializeDelegate`
  (params (Component :type "ControlRigComponent Object Reference"))
  (`self.InitMembers`)
  (`self.OffsetMembers`)
  (`ControlRigComponent.AddMappedCompleteSkeletalMesh` Component (`self.Mesh`))
  (goto _label :!via `Reset`))

(event `self.ControlRig.OnPostForwardsSolveDelegate`
  (params (Component :type "ControlRigComponent Object Reference"))
  (`/Engine/EditorBlueprintResources/StandardMacros.DoOnce` false :!label _label
    (:`Completed`
      ;[0.2719 0.2719 0.2719 0.552] ???
      (`KismetSystemLibrary.DelayUntilNextTick`)
      (`KismetSystemLibrary.DelayUntilNextTick`)
      (`KismetSystemLibrary.DelayUntilNextTick`)
      (`self.AttachMembers`))))

(fn `UserConstructionScript`
  (`self.InitMesh`))