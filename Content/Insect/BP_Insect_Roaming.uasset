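; BP_Insect_Roaming is an insect Blueprint that belongs to a nest, referenced through NestRef.
; Its Die event triggers OnDie, which notifies the nest of the insect's death and then destroys the actor.
; The construction script only calls the parent's, and a navigation path-length check is left unconnected in the event graph.
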(event `Die`
  (`self.OnDie`))

(event `OnDie`
  (`/Game/Insect/Nest/BP_Nest.OnInsectDie` (`self.NestRef`) self)
  (`self.K2_DestroyActor`))

(fn `UserConstructionScript`
  (`parent.UserConstructionScript`))