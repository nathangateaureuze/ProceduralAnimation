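; Player character with Enhanced Input movement, camera, jump and clamped spring-arm zoom, plus interact and attack dispatchers.
; InitWeapon clears attack bindings and hand meshes, then constructs a WeaponClass object that assigns its own event and mesh, keeping weapon logic modular.
; Debug keys swap two weapon classes, toggle walk speed and hold strafe rotation through ControllerState.
; Weapon attack events only print placeholders, and the hand-position aiming code is disconnected.
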(event Custom|InitEquipment
  ;[0.5658 0 1] Equipment
  (CallFunction|InitWeapon))

(event Custom|InitWeapon
  ;[0.5658 0 1] Equipment
  ;;[0.05098 0.05098 0.05098 1 14] Resets
  (EventDispatchers|UnbindallEventsfromAttack)
  (Components|StaticMesh|SetStaticMesh (Variables|Default|GetItem_L) 0)
  (Components|StaticMesh|SetStaticMesh (Variables|Default|GetItem_R) 0)
  (bind _returnvalue (Game|ConstructObjectfromClass (Variables|Default|GetWeapon_Class) self))
  (bind _output_get (Variables|Default|SetWeapon _returnvalue))
  (Default|AssignEvent _output_get)
  (Default|SetMesh _output_get))

(event Input|EnhancedActionEvents|EnhancedInputActionIA_Move
  (params (ActionValue :type Vector%202D%20Structure) (ElapsedSeconds :type Float%20%28double-precision%29) (TriggeredSeconds :type Float%20%28double-precision%29) (InputAction :type Input%20Action%20Object%20Reference :default "/Game/GameMode/Inputs/IA_Move.IA_Move"))
  (bind _returnvalue (Pawn|GetControlRotation :!class /Script/Engine.Pawn))
  ;[1 0.3698 0.3698 1 23] Inputs
  (Pawn|Input|AddMovementInput (Math|Vector|GetRightVector (Math|Rotator|MakeRotator (.roll _returnvalue) 0.0 (.yaw _returnvalue))) (.x ActionValue) false)
  (Pawn|Input|AddMovementInput (Math|Vector|GetForwardVector (Math|Rotator|MakeRotator 0.0 0.0 (.yaw (Pawn|GetControlRotation :!class /Script/Engine.Pawn)))) (.y ActionValue) false))

(event Input|EnhancedActionEvents|EnhancedInputActionIA_Camera
  (params (ActionValue :type Vector%202D%20Structure) (ElapsedSeconds :type Float%20%28double-precision%29) (TriggeredSeconds :type Float%20%28double-precision%29) (InputAction :type Input%20Action%20Object%20Reference :default "/Game/GameMode/Inputs/IA_Camera.IA_Camera"))
  ;[1 0.3698 0.3698 1 23] Inputs
  (Pawn|Input|AddControllerYawInput (.x ActionValue))
  (Pawn|Input|AddControllerPitchInput (.y ActionValue)))

(event Input|EnhancedActionEvents|EnhancedInputActionIA_Jump
  (params (ActionValue :type Boolean) (ElapsedSeconds :type Float%20%28double-precision%29) (TriggeredSeconds :type Float%20%28double-precision%29) (InputAction :type Input%20Action%20Object%20Reference :default "/Game/GameMode/Inputs/IA_Jump.IA_Jump"))
  ;[1 0.3698 0.3698 1 23] Inputs
  (:Started
    (Character|Jump)))

(event Input|EnhancedActionEvents|EnhancedInputActionIA_Zoom
  (params (ActionValue :type Float%20%28double-precision%29) (ElapsedSeconds :type Float%20%28double-precision%29) (TriggeredSeconds :type Float%20%28double-precision%29) (InputAction :type Input%20Action%20Object%20Reference :default "/Game/GameMode/Inputs/IA_Zoom.IA_Zoom"))
  (bind _springarm (Variables|Default|GetSpringArm))
  ;[1 0.3698 0.3698 1 23] Inputs
  (Variables|/Script/Engine.SpringArmComponent|SetTargetArmLength _springarm (Math|Float|Clamp(Float) (+ (* ActionValue (Variables|Camera|GetZoomSensibility)) (Variables|/Script/Engine.SpringArmComponent|GetTargetArmLength _springarm)) (Variables|Camera|GetMinZoom) (Variables|Camera|GetMaxZoom))))

(event Input|EnhancedActionEvents|EnhancedInputActionIA_Attack
  (params (ActionValue :type Boolean) (ElapsedSeconds :type Float%20%28double-precision%29) (TriggeredSeconds :type Float%20%28double-precision%29) (InputAction :type Input%20Action%20Object%20Reference :default "/Game/GameMode/Inputs/IA_Attack.IA_Attack"))
  ;[1 1 1] ATTACK
  (:Started
    (Default|CallAttack)))

(event EventBeginPlay
  ;[1 0.5172 0.09693 1 23] Begin
  (bind _asplayer_controller (Utilities|Casting|CastToPlayerController (Pawn|GetController)))
  (Utilities|IsValid (PlayerController|LocalPlayerSubsystems|GetEnhancedInputLocalPlayerSubsystem _asplayer_controller)
    (:Is%20Valid
      (Input|AddMappingContext (PlayerController|LocalPlayerSubsystems|GetEnhancedInputLocalPlayerSubsystem _asplayer_controller) "/Game/GameMode/Inputs/IMC.IMC" 0 "(bIgnoreAllPressedKeysUntilRelease=True,bForceImmediately=False,bNotifyUserSettings=False)"))
    (:Is%20Not%20Valid
      _))
  (bind _asabp_editor (Utilities|Casting|CastToABP_Editor (Components|SkeletalMesh|GetAnimInstance (Variables|Character|GetMesh))))
  (Variables|Default|SetAnimBP _asabp_editor)
  (CallFunction|InitEquipment))

(event Input|KeyboardEvents|DebugKeyT
  (params (Key :type Key%20Structure :default "None") (ActionValue :type Input%20Action%20Value%20Structure))
  (bind _charactermovement (Variables|Character|GetCharacterMovement))
  (:Released
    (Utilities|FlowControl|FlipFlop
      (:A
        (Variables|/Script/Engine.CharacterMovementComponent|SetMaxWalkSpeed _charactermovement 6e+02))
      (:B
        (Variables|/Script/Engine.CharacterMovementComponent|SetMaxWalkSpeed _charactermovement 1e+02)))))

(event Input|MouseEvents|DebugKeyRightMouseButton
  (params (Key :type Key%20Structure :default "None") (ActionValue :type Input%20Action%20Value%20Structure))
  ;[1 1 1] Strafe
  (:Pressed
    (Utilities|ControllerState true))
  (:Released
    (Utilities|ControllerState false)))

(event Input|KeyboardEvents|DebugKeyY
  (params (Key :type Key%20Structure :default "None") (ActionValue :type Input%20Action%20Value%20Structure))
  ;[0.5658 0 1] Equipment
  (:Pressed
    (Variables|Default|SetWeapon_Class "/Game/Character/Player/Weapon/Weapon_Child1.Weapon_Child1_C")
    (CallFunction|InitEquipment)))

(event Input|KeyboardEvents|DebugKeyU
  (params (Key :type Key%20Structure :default "None") (ActionValue :type Input%20Action%20Value%20Structure))
  ;[0.5658 0 1] Equipment
  (:Pressed
    (Variables|Default|SetWeapon_Class "/Game/Character/Player/Weapon/Weapon_Child2.Weapon_Child2_C")
    (CallFunction|InitEquipment)))

(event Input|KeyboardEvents|E
  (params (Key :type Key%20Structure :default "None"))
  (:Pressed
    (Default|CallInteract)))

(event Custom|Weapon1_Attack
  (Development|PrintString "1" true true "(R=0.000000,G=1.000000,B=0.000000,A=1.000000)"))

(event Custom|Weapon2_Attack
  (Development|PrintString "2" true true "(R=0.000000,G=1.000000,B=0.000000,A=1.000000)"))

(fn ConstructionScript)